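; A plate actor that can be picked up and dropped by a wand and plays a breaking-glass sound on impact.
; Pickup disables physics and attaches it to the given component; drop re-enables physics, detaches with a small upward impulse and resets the sound's DoOnce.
; Hits from PlayerPawnInterface implementers are ignored.
; On BeginPlay it binds to the first Bp_flush's clean-plates event, which destroys the plate mesh component.
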(event `self.ReceiveHit`
  (params (MyComp :type "PrimitiveComponent Object Reference") (Other :type "Actor Object Reference") (OtherComp :type "PrimitiveComponent Object Reference") (bSelfMoved :type Boolean) (HitLocation :type "Vector Structure") (HitNormal :type "Vector Structure") (NormalImpulse :type "Vector Structure") (Hit :type "HitResult Structure (by ref)"))
  ;[1 1 1] play glass sound when dish dropped to ground
  (if (not (`KismetSystemLibrary.DoesImplementInterface` Other "/Game/Assets/player/playerPawnInterface.playerPawnInterface_C"))
    (`/Engine/EditorBlueprintResources/StandardMacros.DoOnce` false :!label _label
      (:`Completed`
        (`GameplayStatics.PlaySoundAtLocation` "/Game/Assets/audio/Glass_Breaking_Cue.Glass_Breaking_Cue" HitLocation)))))

(event `/Game/Assets/blueprints/pickupAbleInterface.pickUp`
  (params (actorToAttachTo :type "SceneComponent Object Reference"))
  ;[1 1 1] attach to wand when pickup
  (`PrimitiveComponent.SetSimulatePhysics` (`self.plate_mesh`) false)
  (`SceneComponent.K2_AttachToComponent` (`self.K2_GetRootComponent`) actorToAttachTo "None" "KeepWorld" "KeepWorld" "KeepWorld" true))

(event `/Game/Assets/blueprints/pickupAbleInterface.dropOff`
  ;[1 1 1] drop from wand
  (`PrimitiveComponent.SetSimulatePhysics` (`self.plate_mesh`) true)
  (`self.K2_DetachFromActor` "KeepWorld" "KeepWorld" "KeepWorld")
  (`PrimitiveComponent.AddImpulse` (`self.plate_mesh`) (0.0 0.0 20.0) "None" false)
  (goto _label :!via `Reset`))

(event `self.ReceiveBeginPlay`
  ;[1 1 1] bind to reset plate event
  (bind _outactors (`GameplayStatics.GetAllActorsOfClass` "/Game/Assets/blueprints/bp_flush.bp_flush_C"))
  (bind _output_get (set `self.ButtonPopper` (`KismetArrayLibrary.Array_Get` _outactors)))
  (add `/Game/Assets/blueprints/bp_flush.cleanPlates` _output_get (delegate `cleaned`)))

(event `cleaned`
  ;[1 1 1] destroy this plate
  (`ActorComponent.K2_DestroyComponent` (`self.plate_mesh`)))

(fn `UserConstructionScript`)